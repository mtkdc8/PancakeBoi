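; Trigger actor that plays a configurable voice line once, either at level start or when the Rover enters its sphere.
; On BeginPlay it caches the Game_Manager and, if PlayFromStart is set, immediately hands it the VoiceClip to play.
; Otherwise, the first sphere overlap by a Rover sends the clip to the manager, with a PlayedLine flag blocking repeats.
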(event `self.ReceiveBeginPlay`
  (bind _returnvalue (`GameplayStatics.GetActorOfClass` "/Game/Blueprints/0_Mandatory/Game_Manager.Game_Manager_C"))
  (set `self.Manager Ref` _returnvalue)
  (if (`self.Play From Start`)
    (set `self.Played Line` true)
    (`/Game/Blueprints/0_Mandatory/Game_Manager.Play Voice Line` (`self.Manager Ref`) (`self.Voice Clip`))))

(event `self.Sphere.OnComponentBeginOverlap`
  (params (OverlappedComponent :type "PrimitiveComponent Object Reference") (OtherActor :type "Actor Object Reference") (OtherComp :type "PrimitiveComponent Object Reference") (OtherBodyIndex :type Integer) (bFromSweep :type Boolean) (SweepResult :type "HitResult Structure (by ref)"))
  (if (not (`self.Played Line`))
    (cast `/Game/Blueprints/0_Mandatory/Rover` OtherActor)
    (set `self.Played Line` true)
    (`/Game/Blueprints/0_Mandatory/Game_Manager.Play Voice Line` (`self.Manager Ref`) (`self.Voice Clip`))))

(fn `UserConstructionScript`)