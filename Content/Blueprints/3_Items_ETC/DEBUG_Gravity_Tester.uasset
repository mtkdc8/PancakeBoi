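; A debug actor that visualizes the gravity the Game_Manager computes at its location.
; On BeginPlay it finds the first Game_Manager, then loops every frame through a zero-second Delay.
; Each pass calls CalculateGravity with traces enabled and draws a one-frame debug sphere trace along the gravity direction, its length scaled by gravity strength.
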(event `self.ReceiveBeginPlay`
  (bind _returnvalue (`self.K2_GetActorLocation`))
  (bind _outactors (`GameplayStatics.GetAllActorsOfClass` "/Game/Blueprints/0_Mandatory/Game_Manager.Game_Manager_C"))
  (set `self.Manager Ref` (`|GetArrayItem` _outactors))
  (`KismetSystemLibrary.Delay` 0.0 :!label _label)
  (bind (_gravity_direction _gravity_scale) (`/Game/Blueprints/0_Mandatory/Game_Manager.Calculate Gravity` (`self.Manager Ref`) self false true))
  (`KismetSystemLibrary.SphereTraceSingle` :`Start` _returnvalue :`End` (+ _returnvalue (* _gravity_direction (* 50 _gravity_scale))) :`Radius` 5.0 :`TraceChannel` "TraceTypeQuery1" :`DrawDebugType` "ForOneFrame" :`TraceHitColor` (struct :`R` 1.0 :`A` 1.0))
  (goto _label))

(fn `UserConstructionScript`)