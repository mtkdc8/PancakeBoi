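; Syrup bottle collectible that the Rover picks up by overlapping its collider.
; A looping timeline spins the cube around yaw from BeginPlay; a height-bob node exists but never runs.
; On the first Rover overlap it notifies the Rover's manager, sets a collected flag, activates the collect effect and scales the cube along a shrink timeline.
; When shrinking finishes, it sets hidden-in-game to false, so the actor is not hidden.
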(event `self.Collider.OnComponentBeginOverlap`
  (params (OverlappedComponent :type "PrimitiveComponent Object Reference") (OtherActor :type "Actor Object Reference") (OtherComp :type "PrimitiveComponent Object Reference") (OtherBodyIndex :type Integer) (bFromSweep :type Boolean) (SweepResult :type "HitResult Structure (by ref)"))
  (if (not (`self.Collected`))
    (bind _asrover (cast `/Game/Blueprints/0_Mandatory/Rover` OtherActor))
    (`/Game/Blueprints/0_Mandatory/Game_Manager.Syrup Bottle Collected` (`/Game/Blueprints/0_Mandatory/Rover.Manager Ref` _asrover))
    (set `self.Collected` true)
    (`ActorComponent.Activate` (`self.Collect_Syrup`) false)
    (bind (_direction _newtrack_0) (`Timeline|Shrink Timeline`)
      (:`Update`
        (bind _returnvalue (* _newtrack_0 0.5))
        (`SceneComponent.SetWorldScale3D` (`self.Cube`) (`KismetMathLibrary.MakeVector` _returnvalue _returnvalue _returnvalue)))
      (:`Finished`
        (`self.SetActorHiddenInGame` false)))))

(event `self.ReceiveBeginPlay`
  (bind (_rotation_roll _rotation_pitch _rotation_yaw) (`KismetMathLibrary.BreakRotator` (`self.Rotation`)))
  (set `self.Rotation` (`SceneComponent.K2_GetComponentRotation` (`self.Cube`)))
  (bind (_direction _newtrack_0) (`Timeline|Timeline` :!label _label)
    (:`Update`
      (`SceneComponent.K2_SetWorldRotation` (`self.Cube`) (`KismetMathLibrary.MakeRotator` _rotation_roll _rotation_pitch (+ (* 180 _newtrack_0) _rotation_yaw)) false false))
    (:`Finished`
      (goto _label :!via `PlayFromStart`))))

(fn `UserConstructionScript`)