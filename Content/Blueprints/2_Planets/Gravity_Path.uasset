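; Gravity_Path is a spline-driven actor that builds a continuous, collidable track mesh along its Path spline.
; The construction script adds one X-forward spline mesh component per segment between neighboring spline points, with query and physics collision.
; Each segment takes its positions, tangents and start and end roll from those points in local space, so the track banks with the spline.
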(fn `UserConstructionScript`
  (bind _path (`self.Path`))
  (bind _path_2 (`self.Path`))
  (bind _returnvalue (`SplineComponent.GetNumberOfSplinePoints` (`self.Path`)))
  (if (>= _returnvalue 2)
    (for _index (range (+ (- _returnvalue 2) 1))
      (bind _returnvalue_2 (`AddComponent|NODE_AddSplineMeshComponent-0` :`RelativeTransform` (`KismetMathLibrary.MakeTransform` (0.0 0.0 0.0) (struct) (1.0 1.0 1.0))))
      (`SplineMeshComponent.SetForwardAxis` _returnvalue_2 "X" true)
      (bind (_returnvalue_roll _returnvalue_pitch _returnvalue_yaw) (`KismetMathLibrary.BreakRotator` (`SplineComponent.GetRotationAtSplinePoint` _path _index "Local")))
      (`SplineMeshComponent.SetStartRoll` _returnvalue_2 _returnvalue_roll true)
      (bind _returnvalue_3 (+ _index 1))
      (bind _returnvalue_roll_2 (`KismetMathLibrary.BreakRotator` (`SplineComponent.GetRotationAtSplinePoint` _path_2 _returnvalue_3 "Local")))
      (`SplineMeshComponent.SetEndRoll` _returnvalue_2 _returnvalue_roll_2 true)
      (`SplineMeshComponent.SetStartAndEnd` _returnvalue_2 (`SplineComponent.GetLocationAtSplinePoint` _path _index "Local") (`SplineComponent.GetTangentAtSplinePoint` _path _index "Local") (`SplineComponent.GetLocationAtSplinePoint` _path_2 _returnvalue_3 "Local") (`SplineComponent.GetTangentAtSplinePoint` _path_2 _returnvalue_3 "Local") true)
      (`PrimitiveComponent.SetCollisionEnabled` _returnvalue_2 "QueryAndPhysics"))))