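; Base planet Blueprint whose construction script sizes and previews the planet's gravity field.
; It derives Radius from half the planet mesh's local X bounds multiplied by its world X scale.
; RadiusVisual is then scaled uniformly from that Radius and GravityReach to show the field's extent, with visibility controlled by ShowGravityFields.
; The file contains only this setup and applies no gravity itself.
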(fn `UserConstructionScript`
  (bind _returnvalue_x (`KismetMathLibrary.BreakVector` (`SceneComponent.K2_GetComponentScale` (`self.Planet Mesh`))))
  (bind (_min _max) (`StaticMeshComponent.GetLocalBounds` (`self.Planet Mesh`)))
  (bind _returnvalue (* (`self.Gravity Reach`) (`self.Radius`) 0.02))
  (`SceneComponent.SetVisibility` (`self.Radius Visual`) (`self.Show Gravity Fields`) false)
  (set `self.Radius` (/ (* _returnvalue_x (`KismetMathLibrary.Abs` (- (.x _min) (.x _max)))) 2.0))
  (`SceneComponent.SetWorldScale3D` (`self.Radius Visual`) (`KismetMathLibrary.MakeVector` _returnvalue _returnvalue _returnvalue)))