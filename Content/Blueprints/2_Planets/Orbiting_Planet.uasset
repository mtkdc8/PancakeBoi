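; Planet actor Blueprint that moves along an orbit around the location where it starts.
; An Orbit timeline, with play rate set by OrbitTime and start offset by PeriodStartTime, supplies a path vector scaled by OrbitRadius.
; Each update rotates that vector by the actor's rotation, so rotation tilts the orbit, and adds the starting location.
; The construction script flattens OrbitVisualizer and scales it to preview the radius.
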(event `self.ReceiveBeginPlay`
  (`TimelineComponent.SetPlayRate` (`self.Orbit`) (/ 1.0 (`self.Orbit Time`)))
  (set `self.Root Location` (`self.K2_GetActorLocation`))
  (`TimelineComponent.SetNewTime` (`self.Orbit`) (`self.Period Start Time`))
  (bind (_direction _location) (`Timeline|Orbit`)
    (:`Update`
      (`self.K2_SetActorRelativeLocation` (+ (`KismetMathLibrary.GreaterGreater_VectorRotator` (* _location (`self.Orbit Radius`)) (`self.K2_GetActorRotation`)) (`self.Root Location`))))))

(fn `UserConstructionScript`
  (bind _returnvalue (/ (`self.Orbit Radius`) 50.0))
  (`parent.UserConstructionScript`)
  (`SceneComponent.SetRelativeScale3D` (`self.Orbit Visualizer`) (`KismetMathLibrary.MakeVector` _returnvalue _returnvalue)))