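; Pancake is one piece of a stack carried by a rover, managed by a manager that activates it with a stack index.
; Each tick it moves by PancakeVelocity and pops off if it drifts too far from the pancake below, or the root for the bottom one.
; Popping detaches it into physics, decrements the rover's count, plays an index-pitched sound, reports losing the last pancake, then loops the manager's custom gravity via Delay(0).
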(event `Activate`
  (params (Manager :type "/Game/Blueprints/0_Mandatory/Game_Manager Object Reference") (Number :type Integer))
  ;[0.7703 0.03704 1] Activation
  (set `self.Manager Ref` Manager)
  (set `self.Pancake Number` Number)
  (set `self.Activated` true)
  (if (!= (`self.Pancake Number`) 0)
    (set `self.Pancake Below Ref` (`|GetArrayItem` (`/Game/Blueprints/0_Mandatory/Game_Manager.Pancakes` (`self.Manager Ref`)) (- (`self.Pancake Number`) 1)))
    (else
      (set `self.Root Location` (`SceneComponent.RelativeLocation` (`self.Hitbox`)))))
  (`self.Begin Pancake Loop`))

(event `Pop Off`
  (bind _rover_ref (`/Game/Blueprints/0_Mandatory/Game_Manager.Rover Ref` (`self.Manager Ref`)))
  ;[1 1 1] Initial Pop Off Logic
  (`PrimitiveComponent.SetSimulatePhysics` (`self.Hitbox`) true)
  (`self.K2_DetachFromActor` "KeepWorld" "KeepWorld" "KeepWorld")
  (set `self.Lost` true)
  (set `/Game/Blueprints/0_Mandatory/Rover.Num Pancakes` (- (`/Game/Blueprints/0_Mandatory/Rover.Num Pancakes` _rover_ref) 1) _rover_ref)
  (`PrimitiveComponent.AddImpulse` (`self.Hitbox`) (* (+ (* (`SceneComponent.GetUpVector` (`self.Hitbox`)) 1.5) (`KismetMathLibrary.Normal` (- (`SceneComponent.RelativeLocation` (`self.Hitbox`)) (`self.Root Location`)))) 300.0) "None" true)
  (`GameplayStatics.PlaySound2D` "/Game/Assets/4_Sounds/Sound_Effects/Lose_Pancake.Lose_Pancake" 1.0 (select `int` (`self.Pancake Number`) :`0` 0.85 :`1` 0.9 :`2` 0.95 :`3` 1.0 :`4` 1.05 :!type "Float (single-precision)") 0.0 null null)
  (if (not (!= (`self.Pancake Number`) 0))
    (`/Game/Blueprints/0_Mandatory/Game_Manager.Lost Last Pancake` (`self.Manager Ref`)))
  ;[0.9686 1 0.4157] Pancake Gravity Loop
  (bind (_gravity_direction _gravity_scale) (`/Game/Blueprints/0_Mandatory/Game_Manager.Calculate Gravity` (`self.Manager Ref`) self false false :!label _label))
  (`PrimitiveComponent.AddForce` (`self.Hitbox`) (* (* _gravity_direction _gravity_scale) 10000.0) "None" false)
  (`KismetSystemLibrary.Delay` 0.0)
  (goto _label))

(event `Begin Pancake Loop`
  ;[0.9686 1 0.4157] Pancake Stack Loop
  (if (not (`self.Lost`)) :!label _label_2
    (`SceneComponent.K2_AddRelativeLocation` (`self.Hitbox`) (`self.Pancake Velocity`) false false)
    (if (== (`self.Pancake Number`) 0)
      (if (> (`KismetMathLibrary.VSize` (- (`self.Root Location`) (`SceneComponent.RelativeLocation` (`self.Hitbox`)))) 50.0)
        _
        (else
          (`KismetSystemLibrary.Delay` 0.0 :!label _label_3)
          (goto _label_2)))
      (elif (> (`KismetMathLibrary.VSize` (- (`SceneComponent.RelativeLocation` (`/Game/Blueprints/0_Mandatory/Pancake.Hitbox` (`self.Pancake Below Ref`))) (`SceneComponent.RelativeLocation` (`self.Hitbox`)))) 40.0)
        _
        (else
          (goto _label_3))))
    (`self.Pop Off`)))

(fn `UserConstructionScript`)