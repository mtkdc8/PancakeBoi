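; Platter_Goal is the level's win goal, playing a victory cutscene once when a Rover enters its trigger.
; It deactivates the Rover, eases it onto RoverSpot with a per-tick Delay loop and yaws itself to match the Rover's camera root.
; The view blends to this actor while the UFOAnimation timeline drives the UFO, lid and camera lerp, with events progressively hiding the Rover and finally the goal effect.
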(event `self.Trigger Box.OnComponentBeginOverlap`
  (params (OverlappedComponent :type "PrimitiveComponent Object Reference") (OtherActor :type "Actor Object Reference") (OtherComp :type "PrimitiveComponent Object Reference") (OtherBodyIndex :type Integer) (bFromSweep :type Boolean) (SweepResult :type "HitResult Structure (by ref)"))
  (bind _platter_ufo (`self.Platter UFO`))
  (bind _invisible_index (`self.Invisible Index`))
  (bind (_relativerotation_roll _relativerotation_pitch _relativerotation_yaw) (`KismetMathLibrary.BreakRotator` (`SceneComponent.RelativeRotation` _platter_ufo)))
  (bind _asrover (cast `/Game/Blueprints/0_Mandatory/Rover` OtherActor))
  (`/Engine/EditorBlueprintResources/StandardMacros.DoOnce` false ; What happens when we win the game
    (:`Completed`
      (bind _output_get (set `self.Rover Ref` _asrover))
      (set `/Game/Blueprints/0_Mandatory/Rover.Activated` false _output_get)
      (`self.Budge Rover Loop`)
      (`PrimitiveComponent.SetCollisionEnabled` (`self.Trigger Box`) "NoCollision")
      (bind (_relativerotation_roll_2 _relativerotation_pitch_2 _relativerotation_yaw_2) (`KismetMathLibrary.BreakRotator` (`SceneComponent.RelativeRotation` (`/Game/Blueprints/0_Mandatory/Rover.Camera Root` _output_get))))
      (`self.K2_SetActorRotation` (`KismetMathLibrary.MakeRotator` 0.0 0.0 _relativerotation_yaw_2) true)
      (bind _output_get_2 (set `self.Original Camera Position` (`SceneComponent.K2_GetComponentToWorld` (`/Game/Blueprints/0_Mandatory/Rover.Camera` (`self.Rover Ref`)))))
      (`SceneComponent.K2_SetWorldTransform` (`self.Victory View`) _output_get_2 false false)
      (`PlayerController.SetViewTargetWithBlend` (`GameplayStatics.GetPlayerController` 0) self 0.0 "VTBlend_Linear" 2.0 false)
      (bind (_direction _lid_height _lid_rotation _actor_location _ufo_spin_speed _camera_lerp) (`Timeline|UFO Animation` :!via `PlayFromStart`)
        (:`Update`
          (`SceneComponent.K2_SetRelativeRotation` _platter_ufo (`KismetMathLibrary.MakeRotator` 0.0 0.0 (+ _relativerotation_yaw _ufo_spin_speed)) false false)
          (`SceneComponent.K2_SetRelativeLocation` (`self.UFO Root`) _actor_location false false)
          (`SceneComponent.K2_SetRelativeLocation` (`self.Platter Lid`) (`KismetMathLibrary.MakeVector` 0.0 0.0 _lid_height) false false)
          (`SceneComponent.K2_SetRelativeRotation` (`self.Platter Lid`) (`KismetMathLibrary.MakeRotator` (.x _lid_rotation) (.y _lid_rotation) (.z _lid_rotation)) false false)
          (`SceneComponent.K2_SetWorldTransform` (`self.Victory View`) (`KismetMathLibrary.TLerp` (`self.Original Camera Position`) (`SceneComponent.K2_GetComponentToWorld` (`self.Camera Target Spot`)) _camera_lerp) false false))
        (:`Make Invisible`
          (`/Game/Blueprints/0_Mandatory/Rover.Make Invisible` (`self.Rover Ref`) _invisible_index)
          (`/Engine/EditorBlueprintResources/StandardMacros.IncrementInt` (`self.Invisible Index`)
            (:`  `
              (if (>= _invisible_index 5)
                (`SceneComponent.SetVisibility` (`self.Platter_Goal_Effect`) false false)))))))))

(event `Budge Rover Loop`
  ;[0.9686 1 0.4157] Move Rover Loop
  (`self.K2_SetActorLocation` (`self.Rover Ref`) (`KismetMathLibrary.VInterpTo` (`self.K2_GetActorLocation` (`self.Rover Ref`)) (`SceneComponent.K2_GetComponentLocation` (`self.Rover Spot`)) (`GameplayStatics.GetWorldDeltaSeconds`) 10.0) false false :!label _label)
  (if (!= (`self.K2_GetActorLocation` (`self.Rover Ref`)) (`SceneComponent.K2_GetComponentLocation` (`self.Rover Spot`)) :`ErrorTolerance` 2.0)
    (`KismetSystemLibrary.Delay` 0.0)
    (goto _label)))

(fn `UserConstructionScript`)