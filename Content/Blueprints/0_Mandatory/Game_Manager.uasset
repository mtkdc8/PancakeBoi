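; Level manager for a rover pancake-delivery game on planets, handling setup, countdown, win/lose flow, star scoring and level loading.
; BeginPlay creates the HUD and UI input pawn, gathers planets, stacks pancakes on the rover and starts a level-specific timer.
; CalculateGravity sums curve-based planet pulls, boosts the nearest and blends toward UniverseCenter, the summed planet positions, when far out.
; A per-frame loop crossfades three audio layers by PlayerDistance.
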(event `self.ReceiveBeginPlay`
  (bind _rover_ref (`self.Rover Ref`))
  (bind _timer (`self.Timer`))
  ;[0.7703 0.03704 1] Begin Play
  ;;[1 1 1] Save Data and Instance references
  (bind _returnvalue (`GameplayStatics.LoadGameFromSlot` "PB"))
  (bind _aspb_save_data (cast `/Game/Save_Data_ETC/PB_Save_Data` _returnvalue)
    (:`then`
      (set `self.Save Data Ref` _aspb_save_data))
    (:`CastFailed`
      (`KismetSystemLibrary.PrintString` "SAVE DATA CAST FAILED - Game Manager" true false (struct :`R` 1.0 :`A` 1.0) 10.0)))
  (bind _aspb_game_instance (cast `/Game/Save_Data_ETC/PB_Game_Instance` (`GameplayStatics.GetGameInstance`))
    (:`then`
      (set `self.Instance Ref` _aspb_game_instance))
    (:`CastFailed`
      (`KismetSystemLibrary.PrintString` "INSTANCE CAST FAILED - Game Manager" true false (struct :`R` 1.0 :`A` 1.0) 10.0)))
  ;;[1 1 1] Spawn Game HUD
  (bind _returnvalue_2 (`|CreateWidget` "/Game/Blueprints/1_HUD/Gameplay_HUD.Gameplay_HUD_C"))
  (`UserWidget.AddToViewport` _returnvalue_2 0)
  (set `self.Game UI Ref` _returnvalue_2)
  (bind _returnvalue_3 (`|SpawnActorFromClass` "/Game/Blueprints/1_HUD/Game_UI_Input.Game_UI_Input_C" (`KismetMathLibrary.MakeTransform` (0.0 0.0 0.0)) "Undefined" "OverrideRootScale" null null))
  (bind _output_get (set `self.Game UI Input Pawn` _returnvalue_3))
  (`/Game/Blueprints/1_HUD/Game_UI_Input.Activate` _output_get self)
  ;;[1 1 1] Spawn Planets
  (bind _outactors (`GameplayStatics.GetAllActorsOfClass` "/Game/Blueprints/2_Planets/Root_Planet.Root_Planet_C"))
  (set `self.All Planets` _outactors)
  ;;[1 1 1] Find Universe Center
  (set `self.Universe Center` (0.0 0.0 0.0))
  (for _array_element (`self.All Planets`)
    (set `self.Universe Center` (+ (`self.Universe Center`) (`self.K2_GetActorLocation` _array_element))))
  ;;[1 1 1] Rover and Pancake Spawning
  (bind _outactors_2 (`GameplayStatics.GetAllActorsOfClass` "/Game/Blueprints/0_Mandatory/Rover.Rover_C"))
  (if (`KismetArrayLibrary.Array_IsValidIndex` _outactors_2)
    (set `self.Rover Ref` (`|GetArrayItem` _outactors_2))
    (for _index (range 5)
      (bind _returnvalue_4 (`|SpawnActorFromClass` "/Game/Blueprints/0_Mandatory/Pancake.Pancake_C" (`KismetMathLibrary.MakeTransform` (+ (`self.K2_GetActorLocation` _rover_ref) (* (`self.GetActorUpVector` _rover_ref) (+ 40.0 (* _index 12.0)))) (`self.K2_GetActorRotation` _rover_ref) (0.8 0.8 0.1)) "Undefined" "OverrideRootScale" null null))
      (`KismetArrayLibrary.Array_Add` (`self.Pancakes`) _returnvalue_4)
      (`self.K2_AttachToComponent` _returnvalue_4 (`/Game/Blueprints/0_Mandatory/Rover.Dish` (`self.Rover Ref`)) "None" "KeepWorld" "KeepWorld" "KeepWorld" true)
      (`/Game/Blueprints/0_Mandatory/Pancake.Activate` _returnvalue_4 self _index)
      ;;[1 1 1] Countdown Timer
      (bind _returnvalue_5 (`GameplayStatics.GetCurrentLevelName` true))
      (bind _returnvalue_6 (`KismetStringLibrary.GetCharacterAsNumber` (`KismetStringLibrary.GetSubstring` _returnvalue_5 6)))
      (if (> _returnvalue_6 9)
        (bind _output_get_2 (set `self.Rec Time` 300))
        (`TimelineComponent.SetPlayRate` _timer (/ 1.0 (`KismetMathLibrary.Conv_IntToDouble` _output_get_2)))
        (else
          (bind _output_get_3 (set `self.Rec Time` (`.IdealTime_14_D8EE2E6D4B307D823DFC8DAF61D88FD6` (break `/Game/Blueprints/1_HUD/Level_Metadata` (`|GetArrayItem` (`/Game/Save_Data_ETC/PB_Game_Instance.Level Metadata` (`self.Instance Ref`)) _returnvalue_6)))))
          (`TimelineComponent.SetPlayRate` _timer (/ 1.0 (`KismetMathLibrary.Conv_IntToDouble` _output_get_3)))))
      (`TimelineComponent.ReverseFromEnd` _timer))
    (`/Game/Blueprints/0_Mandatory/Rover.Activate` (`self.Rover Ref`) self)
    (`self.Begin Music Loops`)))

(event `Stop Timer`
  (`TimelineComponent.Stop` (`self.Timer`)))

(event `Syrup Bottle Collected`
  (`/Game/Blueprints/1_HUD/Gameplay_HUD.Show Collected Syrup` (`self.Game UI Ref`))
  (set `self.Collected Syrup` true))

(event `Win Processes`
  (set `self.Won Level` true)
  (`self.Calculate Stars`)
  (`/Game/Blueprints/1_HUD/Gameplay_HUD.Win Level Processes` (`self.Game UI Ref`) (`self.Star Score`))
  (`Controller.Possess` (`GameplayStatics.GetPlayerController` 0) (`self.Game UI Input Pawn`)))

(event `Reload Level`
  (bind _returnvalue (`GameplayStatics.GetCurrentLevelName` true))
  (`GameplayStatics.OpenLevel` (`KismetStringLibrary.Conv_StringToName` _returnvalue)))

(event `Lost Last Pancake`
  (`self.Stop Timer`)
  (`self.Halt Rover Movement`)
  (`KismetSystemLibrary.Delay` 1.0)
  (`self.Lose Processes`))

(event `Begin Music Loops`
  (bind _orbit_music (`self.Orbit Music`))
  (bind _player_distance (`self.Player Distance`))
  (bind _returnvalue (`KismetMathLibrary.FClamp` (/ (- _player_distance 850.0) 634.0)))
  ;[0.9686 1 0.4157] Music Loop
  (`AudioComponent.FadeIn` (`self.Music`) 0.2 1.0 0.0 "Linear")
  (`AudioComponent.Play` (`self.Orbit Noise`) 0.0)
  (set `self.Target BGM Sounds` (`|MakeArray` (`KismetMathLibrary.Lerp` 1.0 0.0 _returnvalue) _returnvalue (`KismetMathLibrary.SelectFloat` 1.0 0.0 (and (> _player_distance 1684.0) (== (`AudioComponent.VolumeMultiplier` (`self.Music`)) 0.0)))) :!label _label)
  (for (_array_element _array_index) (`|MakeArray` (`self.Music`) (`self.Orbit Noise`) (`self.Orbit Music`))
    (bind _volumemultiplier (`AudioComponent.VolumeMultiplier` _array_element))
    (bind _output (`|GetArrayItem` (`self.Target BGM Sounds`) _array_index))
    (bind _returnvalue_2 (> (- _output _volumemultiplier) 0.0))
    (`AudioComponent.SetVolumeMultiplier` _array_element (`KismetMathLibrary.FInterpTo_Constant` _volumemultiplier _output (`GameplayStatics.GetWorldDeltaSeconds`) (select `int` _array_index :`0` (`KismetMathLibrary.SelectFloat` 0.4 0.2 _returnvalue_2) :`1` (`KismetMathLibrary.SelectFloat` 0.2 0.4 _returnvalue_2) :`2` (`KismetMathLibrary.SelectFloat` 0.1 0.6 _returnvalue_2)))))
  (if (and (not (`AudioComponent.IsPlaying` _orbit_music)) (!= (`AudioComponent.VolumeMultiplier` _orbit_music) 0.0))
    (`AudioComponent.Play` (`self.Orbit Music`) 0.0))
  (`KismetSystemLibrary.Delay` 0.0)
  (goto _label))

(event `Lose Processes`
  (`/Game/Blueprints/1_HUD/Gameplay_HUD.Lose Level Processes` (`self.Game UI Ref`))
  (`Controller.Possess` (`GameplayStatics.GetPlayerController` 0) (`self.Game UI Input Pawn`)))

(event `Halt Rover Movement`
  (set `/Game/Blueprints/0_Mandatory/Rover.Activated` false (`self.Rover Ref`)))

(event `Calculate Stars`
  (bind _returnvalue (+ (`KismetMathLibrary.Conv_ByteToInt` (`/Game/Blueprints/0_Mandatory/Rover.Num Pancakes` (`self.Rover Ref`))) (/ (`self.Remaining Time`) 60)))
  (if (`self.Collected Syrup`)
    (bind _result (`/Engine/EditorBlueprintResources/StandardMacros.IncrementInt` _returnvalue)
      (:`  `
        (set `self.Star Score` (/ _result 2))))
    (else
      (set `self.Star Score` (/ _returnvalue 2)))))

(event `Load Next Level`
  (bind _returnvalue (`GameplayStatics.GetCurrentLevelName` true))
  (bind _returnvalue_2 (+ (`KismetStringLibrary.GetCharacterAsNumber` (`KismetStringLibrary.GetSubstring` _returnvalue 6)) 1))
  (if (not (== (`KismetArrayLibrary.Array_Length` (`/Game/Save_Data_ETC/PB_Game_Instance.Level Metadata` (`self.Instance Ref`))) _returnvalue_2))
    (`GameplayStatics.OpenLevel` (`KismetStringLibrary.Conv_StringToName` (`KismetStringLibrary.Concat_StrStr` "Level_" (`KismetStringLibrary.Conv_IntToString` _returnvalue_2))))))

(event `Game UI Confirm`
  (if (`self.Won Level`)
    (`self.Load Next Level`)
    (else
      (`self.Reload Level`))))

(event `Game UI Cancel`
  (`GameplayStatics.OpenLevel` "Menu_Screen"))

(fn `Calculate Gravity`
  (params (Actor :type "Actor Object Reference") (`Closest Only` :type Boolean) (`Gravity Traces` :type Boolean))
  (returns (`Gravity Direction` :type "Vector Structure") (`Gravity Scale` :type "Float (double-precision)") (`Distance to Planet` :type "Float (double-precision)"))
  (locals (`Actor in Question` :type "Actor Object Reference") (`Gravity Dir` :type "Vector Structure" :default (0.0 0.0 -1.0)) (`Gravity Sca` :type "Float (double-precision)" :default 1.0) (`Show Traces` :type Boolean) (`Gravity Sum` :type "Vector Structure") (`Closest Planet Distance` :type "Float (double-precision)" :default -1.0) (`Closest Planet` :type "/Game/Blueprints/2_Planets/Root_Planet Object Reference") (`Only Closest Planet` :type Boolean))
  (bind _closest_planet (`local.Closest Planet`))
  (bind _closest_planet_distance (`local.Closest Planet Distance`))
  (bind _returnvalue (`self.K2_GetActorLocation` (`local.Actor in Question`)))
  (bind _returnvalue_2 (`self.K2_GetActorLocation` (`local.Actor in Question`)))
  (set `local.Actor in Question` Actor)
  (set `local.Only Closest Planet` `Closest Only`)
  (set `local.Show Traces` `Gravity Traces`)
  (`|ExecutionSequence`
    (:`then_0`
      (if (`KismetArrayLibrary.Array_IsValidIndex` (`self.All Planets`))
        ;[1 1 1] Get Closest Planet
        (for _array_element (`self.All Planets`)
          (bind _returnvalue_3 (- (`KismetMathLibrary.VSize` (- (`self.K2_GetActorLocation` (`local.Actor in Question`)) (`self.K2_GetActorLocation` _array_element))) (`/Game/Blueprints/2_Planets/Root_Planet.Radius` _array_element)))
          (bind _returnvalue_4 (`KismetMathLibrary.SelectFloat` 0.0 _returnvalue_3 (< _returnvalue_3 0.0)))
          (if (or (< _returnvalue_4 _closest_planet_distance) (== _closest_planet_distance -1.0))
            (set `local.Closest Planet` _array_element)
            (set `local.Closest Planet Distance` _returnvalue_4)))
        (set `local.Gravity Sum` (0.0 0.0 0.0))
        (for _array_element_2 (`self.All Planets`)
          (if (`local.Only Closest Planet`)
            (bind _returnvalue_5 (== (`local.Closest Planet`) _array_element_2))
            (if _returnvalue_5
              (bind _returnvalue_6 (`self.K2_GetActorLocation` _array_element_2))
              (bind _returnvalue_7 (`KismetMathLibrary.VSize` (- _returnvalue_2 _returnvalue_6)))
              (bind _radius (`/Game/Blueprints/2_Planets/Root_Planet.Radius` _array_element_2))
              (bind _returnvalue_8 (* _radius (`/Game/Blueprints/2_Planets/Root_Planet.Gravity Reach` _array_element_2)))
              (bind _returnvalue_9 (* (`KismetMathLibrary.GetDirectionUnitVector` _returnvalue_2 _returnvalue_6) (* (`CurveFloat.GetFloatValue` (`/Game/Blueprints/2_Planets/Root_Planet.Gravity Curve` _array_element_2) (`KismetMathLibrary.FClamp` (/ (- _returnvalue_7 _radius) (- _returnvalue_8 _radius)))) (`/Game/Blueprints/2_Planets/Root_Planet.Gravity Scale` _array_element_2) (`KismetMathLibrary.SelectFloat` 1.5 1.0 _returnvalue_5))))
              (set `local.Gravity Sum` (+ (`local.Gravity Sum`) _returnvalue_9) :!label _label)
              (if (`local.Show Traces`)
                (`KismetSystemLibrary.SphereTraceSingle` :`Start` _returnvalue :`End` (+ _returnvalue (* _returnvalue_9 50.0)) :`Radius` 5.0 :`TraceChannel` "TraceTypeQuery1" :`DrawDebugType` "ForOneFrame" :`TraceColor` (struct :`G` 1.0 :`A` 1.0))))
            (elif (or _returnvalue_5 (< _returnvalue_7 _returnvalue_8))
              (goto _label))))
        (set `local.Gravity Sca` (`KismetMathLibrary.FClamp` (`KismetMathLibrary.VSize` (`local.Gravity Sum`)) 0.1))
        (set `local.Gravity Dir` (`KismetMathLibrary.Normal` (`KismetMathLibrary.VLerp` (`KismetMathLibrary.Normal` (`local.Gravity Sum`)) (`KismetMathLibrary.GetDirectionUnitVector` (`self.K2_GetActorLocation` (`local.Actor in Question`)) (`self.Universe Center`)) (`KismetMathLibrary.FClamp` (/ (- (`local.Closest Planet Distance`) (* (`/Game/Blueprints/2_Planets/Root_Planet.Radius` _closest_planet) (- (`/Game/Blueprints/2_Planets/Root_Planet.Gravity Reach` _closest_planet) 1.0))) 4000.0)))))))
    (:`then_1`
      (return (`local.Gravity Dir`) (`local.Gravity Sca`) (`local.Closest Planet Distance`)))))

(fn `UserConstructionScript`)