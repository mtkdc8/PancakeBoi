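; Game UI input Blueprint that forwards player confirm and cancel presses to the game manager.
; An Activate event stores the GameManager reference and sets the Activated flag that gates all input.
; Once active, pressing the Jump action calls GameUIConfirm on the manager and pressing Cancel Action calls GameUICancel.
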(event `Activate`
  (params (`Game Manager` :type "/Game/Blueprints/0_Mandatory/Game_Manager Object Reference"))
  (set `self.Game Manager Ref` `Game Manager`)
  (set `self.Activated` true))

(event `InputAction|Jump`
  (params (Key :type "Key Structure"))
  (:`Pressed`
    (if (`self.Activated`)
      (`/Game/Blueprints/0_Mandatory/Game_Manager.Game UI Confirm` (`self.Game Manager Ref`)))))

(event `InputAction|Cancel Action`
  (params (Key :type "Key Structure"))
  (:`Pressed`
    (if (`self.Activated`)
      (`/Game/Blueprints/0_Mandatory/Game_Manager.Game UI Cancel` (`self.Game Manager Ref`)))))

(fn `UserConstructionScript`)