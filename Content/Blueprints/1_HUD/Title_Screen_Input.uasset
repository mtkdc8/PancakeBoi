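; Title screen input handler that turns player input into Up, Down and Select presses on the title screen UI reference.
; The WS axis drives up and down through a small deadzone, while the Jump action triggers select.
; Held input repeats only after a frame-count delay tracked per direction, and leaving that direction resets its timer so the next press fires immediately.
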(event `Check For Down Input`
  (params (`Axis Value` :type "Float (double-precision)"))
  (bind _frames_since_last_s_input (`self.Frames Since Last S Input`))
  (if (and (< `Axis Value` -0.05) (or (> (- (`KismetSystemLibrary.GetFrameCount`) _frames_since_last_s_input) (`KismetMathLibrary.Conv_IntToInt64` (`self.DEADZONE FRAMECOUNT`))) (== _frames_since_last_s_input -1)))
    (set `self.Frames Since Last S Input` (`KismetSystemLibrary.GetFrameCount`))
    (`/Game/Blueprints/1_HUD/Title_Screen_UI.Down Pressed` (`self.Title Screen UI Ref`))))

(event `Check For Up Input`
  (params (`Axis Value` :type "Float (double-precision)"))
  (bind _frames_since_last_w_input (`self.Frames Since Last W Input`))
  (if (and (> `Axis Value` 0.05) (or (> (- (`KismetSystemLibrary.GetFrameCount`) _frames_since_last_w_input) (`KismetMathLibrary.Conv_IntToInt64` (`self.DEADZONE FRAMECOUNT`))) (== _frames_since_last_w_input -1)))
    (set `self.Frames Since Last W Input` (`KismetSystemLibrary.GetFrameCount`))
    (`/Game/Blueprints/1_HUD/Title_Screen_UI.Up Pressed` (`self.Title Screen UI Ref`))))

(event `InputAxis|WS`
  (params (AxisValue :type "Float (single-precision)"))
  (`self.Check For WS Reset` AxisValue)
  (`self.Check For Up Input` AxisValue)
  (`self.Check For Down Input` AxisValue))

(event `InputAction|Jump`
  (params (Key :type "Key Structure"))
  (:`Pressed`
    (`/Game/Blueprints/1_HUD/Title_Screen_UI.Select Pressed` (`self.Title Screen UI Ref`))))

(event `Check For WS Reset`
  (params (`Axis Value` :type "Float (double-precision)"))
  (`|ExecutionSequence`
    (:`then_0`
      (if (< `Axis Value` 0.05)
        (set `self.Frames Since Last W Input` -1)))
    (:`then_1`
      (if (> `Axis Value` -0.05)
        (set `self.Frames Since Last S Input` -1)))))

(fn `UserConstructionScript`)