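; Rover is a player-controlled pawn with movement, camera look and switchable gravity.
; The WS axis event drives forward movement and also polls the AD and camera axes for strafing and sensitivity-scaled yaw and pitch.
; Pressing Q alternates the gravity movement component's direction between up and down through a FlipFlop, starting with up.
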(event `InputAxis|WS`
  (params (AxisValue :type "Float (single-precision)"))
  (bind (_camera_sensitivity_x _camera_sensitivity_y) (`KismetMathLibrary.BreakVector2D` (`self.Camera Sensitivity`)))
  (`self.AddMovementInput` (`self.GetActorForwardVector`) AxisValue)
  (`self.AddMovementInput` (`self.GetActorRightVector`) (`self.GetInputAxisValue`))
  (`self.AddControllerYawInput` (* (`self.GetInputAxisValue`) _camera_sensitivity_x))
  (`self.AddControllerPitchInput` (* (`self.GetInputAxisValue`) _camera_sensitivity_y)))

(event `Key|Q`
  (params (Key :type "Key Structure"))
  (bind _returnvalue (`self.GetGravityMovementComponent`))
  (:`Pressed`
    (`/Engine/EditorBlueprintResources/StandardMacros.FlipFlop`
      (:`A`
        (`GravityMovementComponent.SetGravityDirection` _returnvalue (0.0 0.0 1.0)))
      (:`B`
        (`GravityMovementComponent.SetGravityDirection` _returnvalue (0.0 0.0 -1.0))))))

(fn `UserConstructionScript`)